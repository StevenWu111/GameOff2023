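; One-way door Blueprint with two leaves that swing open and closed through an interact event.
; A box overlap shows a prompt widget, created at BeginPlay, while the player character is inside.
; UnlockDoorInteract removes the prompt, plays a sound and alternates between playing and reversing a timeline.
; A second FlipFlop on the timeline update rotates the left and right leaves in opposite directions on alternating updates.
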(event `self.UnlockDoorInteract`
  ;[0 0 0] TwoSidesDoor Open
  (`Widget.RemoveFromParent` (`self.OneWayDoor`))
  (`GameplayStatics.PlaySound2D` "/Game/Sound/S_OpenDoor.S_OpenDoor" 1.0 1.0 0.0 null null)
  (`/Engine/EditorBlueprintResources/StandardMacros.FlipFlop`
    (:`A`
      (bind (_direction _opentime) (`Timeline|DoorOpen TL` :!via `PlayFromStart` :!label _label)
        (:`Update`
          (`/Engine/EditorBlueprintResources/StandardMacros.FlipFlop`
            (:`A`
              (`SceneComponent.K2_SetRelativeRotation` (`self.DoorL`) (`KismetMathLibrary.MakeRotator` 0.0 0.0 (`KismetMathLibrary.Lerp` 0.0 100.0 _opentime)) false false))
            (:`B`
              (`SceneComponent.K2_SetRelativeRotation` (`self.DoorR`) (`KismetMathLibrary.MakeRotator` 0.0 0.0 (`KismetMathLibrary.Lerp` 0.0 -100.0 _opentime)) false false))))))
    (:`B`
      (goto _label :!via `Reverse`))))

(event `self.ReceiveBeginPlay`
  ;[0 0 0] TwoSidesDoor Open
  (bind _returnvalue (`|CreateWidget` "/Game/pluu/Blueprint/WBP_OpenDoor.WBP_OpenDoor_C"))
  (set `self.OneWayDoor` _returnvalue))

(event `self.Box.OnComponentBeginOverlap`
  (params (OverlappedComponent :type "PrimitiveComponent Object Reference") (OtherActor :type "Actor Object Reference") (OtherComp :type "PrimitiveComponent Object Reference") (OtherBodyIndex :type Integer) (bFromSweep :type Boolean) (SweepResult :type "HitResult Structure (by ref)"))
  ;[0 0 0] TwoSidesDoor Open
  (if (== OtherActor (`GameplayStatics.GetPlayerCharacter` 0))
    (`UserWidget.AddToViewport` (`self.OneWayDoor`) 0)))

(event `self.Box.OnComponentEndOverlap`
  (params (OverlappedComponent :type "PrimitiveComponent Object Reference") (OtherActor :type "Actor Object Reference") (OtherComp :type "PrimitiveComponent Object Reference") (OtherBodyIndex :type Integer))
  ;[0 0 0] TwoSidesDoor Open
  (if (== (`GameplayStatics.GetPlayerCharacter` 0) OtherActor)
    (`Widget.RemoveFromParent` (`self.OneWayDoor`))))

(fn `UserConstructionScript`)