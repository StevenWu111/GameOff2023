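; BP_LockDoor is a locked double door that opens and closes on interaction once PickUpKey has set HasKey.
; The first successful interaction plays an unlock sound, destroys the lock and beam components, then waits briefly.
; Each interaction plays the door sound and flip-flops DoorOpenTL between play and reverse.
; The timeline swings the leaves in opposite yaw directions, with a nested FlipFlop updating left and right on alternate ticks.
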(event `/Game/Blueprint/Doors/BPI_LockDoorInteract.LockDoorInteract`
  ;[0 0 0] TwoSidesDoor Open
  (if (`self.HasKey?`)
    (if (== (`self.DoorOpenedTimes`) 0)
      (bind _output_get (set `self.DoorOpenedTimes` 0))
      (`/Engine/EditorBlueprintResources/StandardMacros.IncrementInt` _output_get
        (:`  `
          (`GameplayStatics.PlaySound2D` "/Game/Sound/S_Unlock.S_Unlock" 1.0 1.0 0.0 null null)
          (`ActorComponent.K2_DestroyComponent` (`self.Lock`))
          (`ActorComponent.K2_DestroyComponent` (`self.LockBeam`))
          (`KismetSystemLibrary.Delay` 1.5))))
    (`GameplayStatics.PlaySound2D` "/Game/Sound/S_OpenDoor.S_OpenDoor" 1.0 1.0 0.0 null null)
    (`/Engine/EditorBlueprintResources/StandardMacros.FlipFlop`
      (:`A`
        (bind (_direction _opentime) (`Timeline|DoorOpen TL` :!via `PlayFromStart` :!label _label)
          (:`Update`
            (`/Engine/EditorBlueprintResources/StandardMacros.FlipFlop`
              (:`A`
                (`SceneComponent.K2_SetRelativeRotation` (`self.DoorL`) (`KismetMathLibrary.MakeRotator` 0.0 0.0 (`KismetMathLibrary.Lerp` 0.0 -100.0 _opentime)) false false))
              (:`B`
                (`SceneComponent.K2_SetRelativeRotation` (`self.DoorR`) (`KismetMathLibrary.MakeRotator` 0.0 0.0 (`KismetMathLibrary.Lerp` 0.0 100.0 _opentime)) false false))))))
      (:`B`
        (goto _label :!via `Reverse`)))))

(event `/Game/Blueprint/Doors/BPI_DoorKey.PickUpKey`
  ;[0 0 0] TwoSidesDoor Open
  (set `self.HasKey?` true))

(fn `UserConstructionScript`)