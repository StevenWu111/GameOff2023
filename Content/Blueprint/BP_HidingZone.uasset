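; BP_HidingZone is a box trigger volume that marks an area where the GameOffCharacter can hide.
; On begin overlap it increments the character's HidingZoneCount and shows UI_Hiding, either on first entry or, when crouch is required, if crouched on entry.
; A counter handles overlapping zones, so the hiding widgets are removed only when the character leaves the last one.
; Crouch state is checked only at the moment of entry.
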(event `self.ReceiveTick`
  (params (DeltaSeconds :type "Float (single-precision)")))

(event `self.BoxComponent.OnComponentBeginOverlap`
  (params (OverlappedComponent :type "PrimitiveComponent Object Reference") (OtherActor :type "Actor Object Reference") (OtherComp :type "PrimitiveComponent Object Reference") (OtherBodyIndex :type Integer) (bFromSweep :type Boolean) (SweepResult :type "HitResult Structure (by ref)"))
  (bind _asgame_off_character (cast `GameOffCharacter` OtherActor))
  (if (`self.bIdCrouchNeeded`)
    (if (`GameOffCharacter.bIsCrouch` _asgame_off_character)
      (bind _hidingzonecount (`GameOffCharacter.HidingZoneCount` _asgame_off_character))
      (bind _returnvalue (+ _hidingzonecount 1))
      (set `GameOffCharacter.HidingZoneCount` _returnvalue _asgame_off_character :!label _label)
      (bind _returnvalue_2 (`|CreateWidget` "/Game/UI/UI_Hiding.UI_Hiding_C"))
      (`UserWidget.AddToViewport` _returnvalue_2 0)
      (else
        (set `GameOffCharacter.HidingZoneCount` _returnvalue _asgame_off_character :!label _label_2)))
    (elif (== _hidingzonecount 0)
      (goto _label)
      (else
        (goto _label_2)))))

(event `self.BoxComponent.OnComponentEndOverlap`
  (params (OverlappedComponent :type "PrimitiveComponent Object Reference") (OtherActor :type "Actor Object Reference") (OtherComp :type "PrimitiveComponent Object Reference") (OtherBodyIndex :type Integer))
  (bind _asgame_off_character (cast `GameOffCharacter` OtherActor))
  (bind _hidingzonecount (`GameOffCharacter.HidingZoneCount` _asgame_off_character))
  (if (== _hidingzonecount 1)
    (bind _returnvalue (- _hidingzonecount 1))
    (set `GameOffCharacter.HidingZoneCount` _returnvalue _asgame_off_character)
    (bind _foundwidgets (`WidgetBlueprintLibrary.GetAllWidgetsOfClass` "/Game/UI/UI_Hiding.UI_Hiding_C"))
    (for _array_element _foundwidgets
      (`Widget.RemoveFromParent` _array_element))
    (else
      (set `GameOffCharacter.HidingZoneCount` _returnvalue _asgame_off_character))))

(fn `UserConstructionScript`)